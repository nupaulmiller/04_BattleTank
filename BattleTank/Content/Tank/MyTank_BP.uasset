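; MyTank_BP is a controllable tank Blueprint that translates player input into movement, camera rotation and firing.
; On BeginPlay it prints a debug message, then initializes TankAiming with the barrel and turret and TankMovement with both tracks.
; Move, turn and fire inputs are delegated to those components, while aim axes rotate the azimuth gimbal and spring arm separately, scaled by delta time.
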(event `self.ReceiveBeginPlay`
  (`KismetSystemLibrary.PrintString` "Saith -> Tank BP Begin Play" true true (struct :`G` 1.0 :`B` 0.07451 :`A` 1.0))
  (`|ExecutionSequence`
    (:`then_0`
      (`TankAimingComponent.Initialize` (`self.Tank Aiming`) (`self.Barrel`) (`self.TankTorret`)))
    (:`then_1`
      (`TankMovementComponent.Initialize` (`self.Tank Movement`) (`self.LeftTrack`) (`self.RightTrack`)))))

(event `InputAxis|AimAzimuth`
  (params (AxisValue :type "Float (single-precision)"))
  ;[1 1 1] Aim Input Controller
  (`SceneComponent.K2_AddLocalRotation` (`self.Azimuth Gimble`) (`KismetMathLibrary.MakeRotator` 0.0 0.0 (* AxisValue (`GameplayStatics.GetWorldDeltaSeconds`) 100.0)) false false))

(event `InputAxis|AimElevation`
  (params (AxisValue :type "Float (single-precision)"))
  ;[1 1 1] Aim Input Controller
  (`SceneComponent.K2_AddLocalRotation` (`self.SpringArm`) (`KismetMathLibrary.MakeRotator` 0.0 (* AxisValue (`GameplayStatics.GetWorldDeltaSeconds`) 100.0)) false false))

(event `InputAction|Fire`
  (params (Key :type "Key Structure"))
  ;[1 1 1] Aim Input Controller
  (:`Pressed`
    (`TankAimingComponent.Fire` (`self.Tank Aiming`))))

(event `InputAxis|Move Forward`
  (params (AxisValue :type "Float (single-precision)"))
  ;[1 1 1] Input
  (`TankMovementComponent.IntendMoveForward` (`self.Tank Movement`) AxisValue))

(event `InputAxis|Turn Right`
  (params (AxisValue :type "Float (single-precision)"))
  ;[1 1 1] Input
  (`TankMovementComponent.IntendTurnRight` (`self.Tank Movement`) AxisValue))

(fn `UserConstructionScript`)